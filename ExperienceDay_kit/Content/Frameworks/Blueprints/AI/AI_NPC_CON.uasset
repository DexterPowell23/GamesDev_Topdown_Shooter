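; AI controller for NPC tanks that runs the AI_NPC behavior tree on BeginPlay.
; On each perception update, a BP_Player actor flagged IsPlayer is written to the blackboard Target key and to the controlled BP_Tank's target variable.
; Any other actor clears both, and the update never checks whether the stimulus was sensed or lost.
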(event `self.ReceiveBeginPlay`
  (`self.RunBehaviorTree` "/Game/Frameworks/Blueprints/AI/AI_NPC.AI_NPC"))

(event `self.AIPerception.OnTargetPerceptionUpdated`
  (params (Actor :type "Actor Object Reference") (Stimulus :type "AIStimulus Structure"))
  (bind _returnvalue (`AIBlueprintHelperLibrary.GetBlackboard` null))
  (bind _returnvalue_2 (`self.K2_GetPawn`))
  (bind _asbp_player (cast `/Game/Frameworks/Blueprints/Data/BP_Player` Actor)
    (:`then`
      (if (`/Game/Frameworks/Blueprints/Data/BP_Player.IsPlayer` _asbp_player)
        (`BlackboardComponent.SetValueAsObject` _returnvalue "Target" _asbp_player)
        (bind _asbp_tank (cast `/Game/Frameworks/Blueprints/WorldBlueprints/NPC/BP_Tank` _returnvalue_2))
        (set `/Game/Frameworks/Blueprints/WorldBlueprints/NPC/BP_Tank.Taget` _asbp_player _asbp_tank)
        (else
          (`BlackboardComponent.SetValueAsObject` _returnvalue "Target" null :!label _label)
          (bind _asbp_tank_2 (cast `/Game/Frameworks/Blueprints/WorldBlueprints/NPC/BP_Tank` _returnvalue_2))
          (set `/Game/Frameworks/Blueprints/WorldBlueprints/NPC/BP_Tank.Taget` null _asbp_tank_2))))
    (:`CastFailed`
      (goto _label))))

(fn `UserConstructionScript`)