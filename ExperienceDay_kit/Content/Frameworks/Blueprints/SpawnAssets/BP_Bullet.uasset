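; BP_Bullet is a bullet actor that applies damage and a physical impulse on contact.
; Sphere handles hits and Sphere1 handles overlaps, both ignoring the actor stored in Owener and otherwise calling ApplyDamage with BulletDamage, then firing the RadialForce impulse.
; The hit path leaves DamagedActor unconnected, so only the overlap path passes a damage target.
; Neither path destroys the bullet.
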(event `self.Sphere1.OnComponentBeginOverlap`
  (params (OverlappedComponent :type "PrimitiveComponent Object Reference") (OtherActor :type "Actor Object Reference") (OtherComp :type "PrimitiveComponent Object Reference") (OtherBodyIndex :type Integer) (bFromSweep :type Boolean) (SweepResult :type "HitResult Structure (by ref)"))
  (bind _owener (`self.Owener`))
  (if (not (== OtherActor _owener))
    (`GameplayStatics.ApplyDamage` OtherActor (`self.Bullet Damage`) null _owener)
    (`RadialForceComponent.FireImpulse` (`self.RadialForce`))))

(event `self.Sphere.OnComponentHit`
  (params (HitComponent :type "PrimitiveComponent Object Reference") (OtherActor :type "Actor Object Reference") (OtherComp :type "PrimitiveComponent Object Reference") (NormalImpulse :type "Vector Structure") (Hit :type "HitResult Structure (by ref)"))
  (bind _owener (`self.Owener`))
  (if (not (== OtherActor _owener))
    (`GameplayStatics.ApplyDamage` null (`self.Bullet Damage`) null _owener)
    (`RadialForceComponent.FireImpulse` (`self.RadialForce`))))

(fn `UserConstructionScript`)