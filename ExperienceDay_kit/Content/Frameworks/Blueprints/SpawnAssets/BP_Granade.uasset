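; BP_Granade is a timed grenade that counts down and then explodes.
; A looping one-second timer decrements a clamped Time value; at zero it spawns BP_Boom at its location, passing on owner and explosion damage, then destroys itself.
; Tick pushes the remaining time into a UI_Timer widget component for display.
; Sphere overlap and hit events are empty, and the delayed collision and physics toggles are unconnected.
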(event `self.ReceiveTick`
  (params (DeltaSeconds :type "Float (single-precision)"))
  (bind _asui_timer (cast `/Game/Frameworks/Blueprints/UI/UI_Timer` (`WidgetComponent.GetUserWidgetObject` (`self.Widget`))))
  (set `/Game/Frameworks/Blueprints/UI/UI_Timer.Timer` (`self.Time`) _asui_timer))

(event `self.ReceiveBeginPlay`
  (`KismetSystemLibrary.K2_SetTimerDelegate` (delegate `Timer`) 1.0 true))

(event `self.Sphere1.OnComponentBeginOverlap`
  (params (OverlappedComponent :type "PrimitiveComponent Object Reference") (OtherActor :type "Actor Object Reference") (OtherComp :type "PrimitiveComponent Object Reference") (OtherBodyIndex :type Integer) (bFromSweep :type Boolean) (SweepResult :type "HitResult Structure (by ref)")))

(event `Timer`
  (bind _output_get (set `self.Time` (`KismetMathLibrary.Clamp` (- (`self.Time`) 1) 0 5)))
  (if (== _output_get 0)
    (`|SpawnActorFromClass` "/Game/Frameworks/Blueprints/SpawnAssets/BP_Boom.BP_Boom_C" (`KismetMathLibrary.MakeTransform` (`self.K2_GetActorLocation`)) "AlwaysSpawn" "MultiplyWithRoot" null (`self.Owener`) (`self.Explosion Damage`) null)
    (`self.K2_DestroyActor`)))

(event `self.Sphere1.OnComponentHit`
  (params (HitComponent :type "PrimitiveComponent Object Reference") (OtherActor :type "Actor Object Reference") (OtherComp :type "PrimitiveComponent Object Reference") (NormalImpulse :type "Vector Structure") (Hit :type "HitResult Structure (by ref)")))

(fn `UserConstructionScript`)