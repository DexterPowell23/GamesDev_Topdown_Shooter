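; BP_Boom is an explosion actor that applies damage to any actor overlapping its sphere, crediting a stored owner as damage causer.
; If the victim is a BP_Player with zero HP afterwards, its mesh switches to physics simulation.
; A Boom_Damage timeline would grow the sphere and radial force, fire impulses and then destroy the actor, but nothing in the graph starts it.
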(event `self.Sphere.OnComponentBeginOverlap`
  (params (OverlappedComponent :type "PrimitiveComponent Object Reference") (OtherActor :type "Actor Object Reference") (OtherComp :type "PrimitiveComponent Object Reference") (OtherBodyIndex :type Integer) (bFromSweep :type Boolean) (SweepResult :type "HitResult Structure (by ref)"))
  (`GameplayStatics.ApplyDamage` OtherActor (`self.Explosion Damage`) null (`self.Owener`))
  (bind _asbp_player (cast `/Game/Frameworks/Blueprints/Data/BP_Player` OtherActor))
  (if (== (`/Game/Frameworks/Blueprints/Data/BP_Player.HP` _asbp_player) 0.0)
    (`PrimitiveComponent.SetSimulatePhysics` (`Character.Mesh` _asbp_player) true)))

(fn `UserConstructionScript`)