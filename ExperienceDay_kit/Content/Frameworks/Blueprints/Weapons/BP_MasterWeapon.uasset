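; Master weapon actor that configures itself on BeginPlay from the DB_Weapons row matching its Weapon enum.
; Update builds mesh, muzzle and eject Niagara effects from socket names, plus extras for mini-gun, flamethrower, grenade and rocket launchers.
; Equipping attaches it and any backpack to the owner's mesh and binds the owner's Fire event to shooting.
; Shots spend ammo and spawn bullets, cycling fire-point sockets; Tick syncs mini-gun ammo display actor.
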(event `TriggerClicked_Event`)

(event `self.ReceiveTick`
  (params (DeltaSeconds :type "Float (single-precision)"))
  (`TimelineComponent.SetPlayRate` (`self.Mini-Gun`) (`self.MiniGunSpeed`))
  (bind _as_bp_mini_gun_ammo (`self.As BP Mini Gun Ammo`)
    (:`then`
      (set `/Game/Frameworks/Blueprints/Weapons/BP_Mini_Ammo.Ammo` (`self.CurrentAmmo`) _as_bp_mini_gun_ammo))
    (:`else`)))

(event `Shoot_Event`
  (bind _currentammo (`self.CurrentAmmo`))
  (bind _component (`self.Component`))
  (bind (_meshes _max_ammo _ammo_storage _fire_points _bullet) (break `/Game/Frameworks/Blueprints/Data/Str_Weapons` (`self.WeaponData`)))
  (bind _output (`|GetArrayItem` (`self.FirePoints`) (`self.SocketIndex`)))
  (bind _output_2 (`|GetArrayItem` (`self.Flash`) (`self.SocketIndex`)))
  (if (not (== _currentammo 0))
    (if (> _fire_points 1)
      (set `self.SocketIndex` (`KismetMathLibrary.Clamp` (+ (`self.SocketIndex`) 1) 0 _fire_points)))
    (set `self.IsFiring` true)
    (set `self.CurrentAmmo` (`KismetMathLibrary.Clamp` (- _currentammo 1) 0 _max_ammo))
    (`|SpawnActorFromClass` _bullet (`KismetMathLibrary.MakeTransform` (`SceneComponent.GetSocketLocation` _component _output) (`SceneComponent.GetSocketRotation` _component _output)) "AlwaysSpawn" "MultiplyWithRoot" null null)
    (`/Engine/EditorBlueprintResources/StandardMacros.IsValid` _output_2
      (:`Is Valid`
        (`ActorComponent.Activate` _output_2 true)
        (`ActorComponent.Activate` (`self.EjectFx`) true))
      (:`Is Not Valid`
        _))
    (set `self.IsFiring` false)
    (if (and (== (`self.SocketIndex`) _fire_points) (> _fire_points 1))
      (set `self.SocketIndex` 0))))

(event `self.ReceiveBeginPlay`
  (`self.Update`)
  (add `self.EquipWeapon` (delegate `EquipWeapon_Event`)))

(event `EquipWeapon_Event` :!signature `self.EquipWeapon`
  (params (Owner :type "/Game/Frameworks/Blueprints/Data/BP_Player Object Reference") (Socket :type Name) (Pack :type Name))
  (bind _mesh (`Character.Mesh` Owner))
  (bind _packattachment (`self.PackAttachment`))
  (bind _packattachment_2 (`self.PackAttachment`))
  (add `/Game/Frameworks/Blueprints/Data/BP_Player.Fire` Owner (delegate `Shoot_Event`))
  (`PrimitiveComponent.SetCollisionEnabled` (`self.Handle`) "NoCollision")
  (`PrimitiveComponent.SetCollisionEnabled` (`self.Attachment`) "NoCollision")
  (`self.K2_AttachToComponent` _mesh Socket "SnapToTarget" "SnapToTarget" "KeepRelative")
  (switch `/Game/Frameworks/Blueprints/Data/WeaponList` (`self.Weapon`)
    (:`NewEnumerator8`
      (`StaticMeshComponent.SetStaticMesh` _packattachment "/Game/Frameworks/Assets/Weapons/Meshes/SM_Pack.SM_Pack")
      (`SceneComponent.K2_AttachToComponent` _packattachment _mesh Pack "SnapToTarget" "SnapToTarget" "KeepWorld" true)
      (`SceneComponent.SetVisibility` _packattachment_2 true false))
    (:`NewEnumerator12`
      (`StaticMeshComponent.SetStaticMesh` _packattachment "/Game/Frameworks/Assets/Weapons/Meshes/SM_FlameThrower_Pack.SM_FlameThrower_Pack")
      (`SceneComponent.K2_AttachToComponent` _packattachment _mesh Pack "SnapToTarget" "SnapToTarget" "KeepWorld" true)
      (`SceneComponent.SetVisibility` _packattachment_2 true false)
      (`SceneComponent.SetVisibility` (`self.Cable`) true false))))

(event `UnEquipWeapon_Event`
  (params (Owner :type "/Game/Frameworks/Blueprints/Data/BP_Player Object Reference")))

(event `Update`
  (bind _weapon (`self.Weapon`))
  (bind _component (`self.Component`))
  (bind _cable (`self.Cable`))
  (if (`|EnumEquality` _weapon "NewEnumerator8")
    (set `self.Component` (`self.Attachment`))
    (else
      (set `self.Component` (`self.Handle`))))
  (bind _returnvalue (`|GetDataTableRow` "/Game/Frameworks/Blueprints/Data/DB_Weapons.DB_Weapons" (`KismetStringLibrary.Conv_StringToName` (`|GetEnumeratorNameAsString` _weapon)))
    (:`then`
      (bind _output_get (set `self.WeaponData` _returnvalue))
      (bind (_meshes _max_ammo _ammo_storage _fire_points _bullet _muzzleflash _ejectfx) (break `/Game/Frameworks/Blueprints/Data/Str_Weapons` _output_get))
      (set `self.CurrentAmmo` _max_ammo)
      (`|ExecutionSequence`
        (:`then_0`
          (`StaticMeshComponent.SetStaticMesh` (`self.Handle`) _meshes))
        (:`then_1`
          (for _index (range 1 (+ _fire_points 1))
            (bind _returnvalue_2 (`KismetStringLibrary.Conv_StringToName` (`KismetTextLibrary.Conv_TextToString` (`|FormatText` "FirePoint_0{0}" _index))))
            (`KismetArrayLibrary.Array_Add` (`self.FirePoints`) _returnvalue_2)
            (bind _returnvalue_3 (`AddComponent|NODE_AddArrowComponent-1` :`bManualAttachment` true :`RelativeTransform` (`KismetMathLibrary.MakeTransform` (`SceneComponent.GetSocketLocation` _component _returnvalue_2) (`SceneComponent.GetSocketRotation` _component _returnvalue_2))))
            (bind _returnvalue_4 (`AddComponent|NODE_AddNiagaraComponent-1` :`bManualAttachment` true))
            (`NiagaraComponent.SetAsset` _returnvalue_4 _muzzleflash true)
            (`SceneComponent.K2_AttachToComponent` _returnvalue_4 _component _returnvalue_2 "SnapToTarget" "SnapToTarget" "KeepRelative" true)
            (`SceneComponent.K2_AttachToComponent` _returnvalue_3 _component _returnvalue_2 "SnapToTarget" "SnapToTarget" "KeepRelative" true)
            (`KismetArrayLibrary.Array_Add` (`self.Flash`) _returnvalue_4)
            (bind _returnvalue_5 (`AddComponent|NODE_AddNiagaraComponent-2` :`bManualAttachment` true))
            (`NiagaraComponent.SetAsset` _returnvalue_5 _ejectfx true)
            (`SceneComponent.K2_AttachToComponent` _returnvalue_5 (`self.Handle`) "EjectPoint" "SnapToTarget" "SnapToTarget" "KeepRelative" true)
            (set `self.EjectFx` _returnvalue_5))
          (switch `/Game/Frameworks/Blueprints/Data/WeaponList` _weapon
            (:`NewEnumerator1`
              (`SceneComponent.K2_AttachToComponent` (`self.Attachment`) (`self.Handle`) "Attachment" "SnapToTarget" "KeepWorld" "KeepRelative" true)
              (`StaticMeshComponent.SetStaticMesh` (`self.Attachment`) "/Game/Frameworks/Assets/Weapons/Meshes/GrenadeLauncher_Wheel.GrenadeLauncher_Wheel"))
            (:`NewEnumerator5`
              (for _index_2 (range 1 (+ (`self.CurrentAmmo`) 1))
                (bind _returnvalue_6 (`AddComponent|NODE_AddStaticMeshComponent-4`))
                (`SceneComponent.K2_AttachToComponent` _returnvalue_6 (`self.Handle`) (`|GetArrayItem` (`self.FirePoints`) _index_2) "SnapToTarget" "KeepWorld" "KeepRelative" true)
                (`KismetArrayLibrary.Array_Add` (`self.CurrentRockets`) _returnvalue_6)))
            (:`NewEnumerator8`
              (`SceneComponent.K2_AttachToComponent` (`self.Attachment`) (`self.Handle`) "Attachment" "SnapToTarget" "KeepRelative" "KeepRelative" true)
              (`StaticMeshComponent.SetStaticMesh` (`self.Attachment`) "/Game/Frameworks/Assets/Weapons/Meshes/SM_Mini-Gun_Wheel.SM_Mini-Gun_Wheel")
              (bind _returnvalue_7 (`|SpawnActorFromClass` "/Game/Frameworks/Blueprints/Weapons/BP_Mini_Ammo.BP_Mini_Ammo_C" (`KismetMathLibrary.MakeTransform` (0.0 0.0 0.0)) "AlwaysSpawn" "MultiplyWithRoot" null (`self.CurrentAmmo`) null))
              (bind _output_get_2 (set `self.As BP Mini Gun Ammo` _returnvalue_7))
              (bind _rootcomponent (`Actor.RootComponent` _output_get_2))
              (`SceneComponent.K2_AttachToComponent` _rootcomponent (`self.Handle`) "Cable" "SnapToTarget" "SnapToTarget" "KeepRelative" true)
              (`SceneComponent.K2_SetRelativeRotation` _rootcomponent (struct :`Yaw` -90.0 :`Roll` 180.0) false false))
            (:`NewEnumerator12`
              (`SceneComponent.K2_AttachToComponent` _cable (`self.Handle`) "Cable" "SnapToTarget" "SnapToTarget" "KeepRelative" true)
              (`SceneComponent.SetVisibility` _cable false false))))))))

(fn `UserConstructionScript`)