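; BP_Mini_Ammo is a weapon ammo belt that shows each round as a mesh in a physics-constrained chain.
; On BeginPlay, ReloadAmmo spawns Ammo meshes spaced by mesh width minus an offset, linking them from StartPoint to EndPoint.
; Tick destroys the last mesh, one per frame, while the chain length differs from Ammo, without re-linking EndPoint.
; The Construction Script holds a disconnected copy of the build logic.
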(event `self.ReceiveBeginPlay`
  (`self.ReloadAmmo`))

(event `self.ReceiveTick`
  (params (DeltaSeconds :type "Float (single-precision)"))
  (bind _ammo_current (`self.Ammo_Current`))
  (bind _output (`|GetArrayItem` _ammo_current (`KismetArrayLibrary.Array_LastIndex` _ammo_current)))
  (if (not (== (`KismetArrayLibrary.Array_Length` (`self.Ammo_Current`)) (`self.Ammo`)))
    (`ActorComponent.K2_DestroyComponent` _output)
    (`KismetArrayLibrary.Array_RemoveItem` _ammo_current _output)))

(event `ReloadAmmo`
  (bind _ammo_current (`self.Ammo_Current`))
  (bind (_min _max) (break `Box` (`StaticMesh.GetBoundingBox` (`self.New Mesh`))))
  (set `self.CellSize` (- (.x (- _max _min)) (`self.DistanceOffSet`)))
  (for _index (range 1 (+ (`self.Ammo`) 1))
    (bind _returnvalue (* _index (`self.CellSize`)))
    (bind _returnvalue_2 (`AddComponent|NODE_AddStaticMeshComponent-2` :`RelativeTransform` (`KismetMathLibrary.MakeTransform` (`KismetMathLibrary.MakeVector` _returnvalue))))
    (if (== _index 1)
      (`PhysicsConstraintComponent.SetConstrainedComponents` (`self.PhysicsConstraint`) (`self.StartPoint`) "None" _returnvalue_2 "None")
      (elif (== _index 2)
        (bind _returnvalue_3 (`AddComponent|NODE_AddPhysicsConstraintComponent-3` :`RelativeTransform` (`KismetMathLibrary.MakeTransform` (`KismetMathLibrary.MakeVector` (`self.CellSize`)))))
        (`PhysicsConstraintComponent.SetConstrainedComponents` _returnvalue_3 _returnvalue_2 "None" (`self.LastComponent`) "None")
        (else
          (bind _returnvalue_4 (`AddComponent|NODE_AddPhysicsConstraintComponent-4` :`RelativeTransform` (`KismetMathLibrary.MakeTransform` (`KismetMathLibrary.MakeVector` _returnvalue))))
          (`PhysicsConstraintComponent.SetConstrainedComponents` _returnvalue_4 (`self.LastComponent`) "None" _returnvalue_2 "None"))))
    (bind _output_get (set `self.LastComponent` _returnvalue_2))
    (`KismetArrayLibrary.Array_Add` (`self.Ammo_Current`) _output_get))
  (`PhysicsConstraintComponent.SetConstrainedComponents` (`self.PhysicsConstraint1`) (`|GetArrayItem` _ammo_current (`KismetArrayLibrary.Array_LastIndex` _ammo_current)) "None" (`self.EndPoint`) "None"))

(fn `UserConstructionScript`)