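; Shared combat character for the player and soldier enemies, handling health, shooting, melee, grenades and death.
; IsPlayer adds aim-marker rotation, HUD and respawn with Score and HasKey; enemies get HP bars, drop pickups and award score to a player killer.
; For non-tank enemies, the construction script uses an optionally random Index to set rank, look, stats and weapons.
; Shoot sphere-traces ahead to choose alternating melee or gunfire montages, looping while fire is held.
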(event `TossGrenade`
  (bind _arrow1 (`self.Arrow1`))
  (`SceneComponent.SetVisibility` (`self.Grenade`) false false)
  (`|SpawnActorFromClass` "/Game/Frameworks/Blueprints/SpawnAssets/BP_Granade.BP_Granade_C" (`KismetMathLibrary.MakeTransform` (`SceneComponent.K2_GetComponentLocation` _arrow1) (`SceneComponent.K2_GetComponentRotation` _arrow1)) "Undefined" "MultiplyWithRoot" null self (`self.Explosion Damage`) 5 null)
  (set `self.Grenade_Current` (`KismetMathLibrary.Clamp` (- (`self.Grenade_Current`) 1) 0 (`self.Grenade_Max`))))

(event `HiddenWeapons`
  (`SceneComponent.SetVisibility` (`self.Gun`) false false)
  (`SceneComponent.SetVisibility` (`self.Melee`) false false))

(event `ShowGrenade`
  (`SceneComponent.SetVisibility` (`self.Grenade`) true false))

(event `StartGreande`
  (if (> (`self.Grenade_Current`) 0)
    (`|PlayMontage` (`self.Mesh`) "/Game/Frameworks/Assets/Characters/Animations/Toss_Grenade_Montage.Toss_Grenade_Montage"
      (:`OnCompleted`
        (`SceneComponent.SetVisibility` (`self.Gun`) true false)))))

(event `self.ReceiveBeginPlay`
  (if (`self.IsPlayer`)
    (`|SpawnActorFromClass` "/Game/Frameworks/Blueprints/SpawnAssets/Aim.Aim_C" (`KismetMathLibrary.MakeTransform` (`self.K2_GetActorLocation`)) "AlwaysSpawn" "MultiplyWithRoot" null null)
    (bind _returnvalue (`|CreateWidget` "/Game/Frameworks/Blueprints/UI/HUD.HUD_C"))
    (`UserWidget.AddToViewport` _returnvalue 0)))

(event `self.ReceiveTick`
  (params (DeltaSeconds :type "Float (single-precision)"))
  (bind _widget_0 (`self.Widget_0`))
  (bind (_returnvalue_roll _returnvalue_pitch _returnvalue_yaw) (`KismetMathLibrary.BreakRotator` (`KismetMathLibrary.FindLookAtRotation` (`self.K2_GetActorLocation`) (`self.K2_GetActorLocation` (`self.Aim_Marker`)))))
  (if (`self.IsPlayer`)
    (`SceneComponent.SetVisibility` _widget_0 false false)
    (else
      (bind _asui_hp_bar (cast `/Game/Frameworks/Blueprints/UI/UI_HP_Bar` (`WidgetComponent.GetUserWidgetObject` _widget_0)))
      (set `/Game/Frameworks/Blueprints/UI/UI_HP_Bar.HP` (`self.HP`) _asui_hp_bar)
      (set `/Game/Frameworks/Blueprints/UI/UI_HP_Bar.Max_HP` (`self.HP_Max`) _asui_hp_bar)
      (set `/Game/Frameworks/Blueprints/UI/UI_HP_Bar.Tile` (`self.Tile`) _asui_hp_bar)))
  (`self.HP_Cheack`)
  (if (`self.IsPlayer`)
    (bind _returnvalue (`GameplayStatics.GetActorOfClass` "/Game/Frameworks/Blueprints/SpawnAssets/Aim.Aim_C"))
    (set `self.Aim_Marker` _returnvalue)
    (if (not (`self.IsDead?`))
      (`self.K2_SetActorRelativeRotation` (`KismetMathLibrary.MakeRotator` 0.0 0.0 _returnvalue_yaw)))))

(event `HP_Cheack`
  (if (== (`self.HP`) 0.0)
    (set `self.IsDead?` true)
    (`CharacterMovementComponent.SetMovementMode` (`self.CharacterMovement`) "MOVE_None" 0)))

(event `Remove_Character`
  (bind _returnvalue (`GameplayStatics.GetPlayerCharacter` 0))
  (if (`self.IsPlayer`)
    (bind _returnvalue_2 (`GameplayStatics.GetActorOfClass` "/Script/Engine.PlayerStart"))
    (bind _returnvalue_3 (`|SpawnActorFromClass` "BP_Player_C" (`KismetMathLibrary.MakeTransform` (`self.K2_GetActorLocation` _returnvalue_2)) "AlwaysSpawn" "MultiplyWithRoot" null null true (`self.Score`) 50.0 40.0 100.0 (`self.HasKey?`) true 0 null))
    (`Controller.Possess` (`GameplayStatics.GetPlayerController` 0) _returnvalue_3)
    (`self.K2_DestroyActor`)
    (else
      (`PrimitiveComponent.SetCollisionEnabled` (`self.CapsuleComponent`) "NoCollision")
      (bind _asbp_top_down_character (cast `/Game/Frameworks/Blueprints/Data/BP_Player` _returnvalue)
        (:`then`
          (if (== (`self.Damage Causer`) _returnvalue)
            (set `/Game/Frameworks/Blueprints/Data/BP_Player.Score` (+ (`/Game/Frameworks/Blueprints/Data/BP_Player.Score` _asbp_top_down_character) 1) _asbp_top_down_character)))
        (:`CastFailed`
          _))
      (`|SpawnActorFromClass` "/Game/Frameworks/Blueprints/WorldBlueprints/BP_Pickup.BP_Pickup_C" (`KismetMathLibrary.MakeTransform` (`self.K2_GetActorLocation`)) "AlwaysSpawn" "MultiplyWithRoot" null "NewEnumerator0" (`|MakeArray` "NewEnumerator0" "NewEnumerator1" "NewEnumerator2" :!type "/Game/Frameworks/Blueprints/Data/Pickup Enum") true null)
      (`self.K2_DestroyActor`))))

(event `self.ReceiveAnyDamage`
  (params (Damage :type "Float (single-precision)") (DamageType :type "DamageType Object Reference") (InstigatedBy :type "Controller Object Reference") (DamageCauser :type "Actor Object Reference"))
  (bind _hp (`self.HP`))
  ;[1 1 1] DamageApply
  (set `self.Damage Causer` DamageCauser)
  (if (not (`self.GettingHit`))
    (set `self.Isattacking` false)
    (if (> _hp 0.0)
      (set `self.HP` (`KismetMathLibrary.FClamp` (- _hp Damage) 0.0 (`self.HP_Max`)))
      (`|PlayMontage` (`self.Mesh`) "/Game/Frameworks/Assets/Characters/Animations/Hit_Reaction_Montage.Hit_Reaction_Montage"
        (:`then`
          (set `self.GettingHit` true))
        (:`OnCompleted`
          (set `self.GettingHit` false :!label _label))
        (:`OnInterrupted`
          (goto _label))))))

(event `Shoot`
  (bind _returnvalue (`self.K2_GetActorLocation`))
  (bind _mesh (`self.Mesh`))
  (if (not (and (`self.IsDead?`) (`self.Isattacking`) (`self.GettingHit`)))
    (set `self.Isattacking` true)
    (bind _outhit (`KismetSystemLibrary.SphereTraceSingle` _returnvalue (+ _returnvalue (* (`self.GetActorForwardVector`) 150.0)) 90.0 "TraceTypeQuery1"))
    (if (`GameplayStatics.BreakHitResult` _outhit)
      (`SceneComponent.SetVisibility` (`self.Melee`) true false :!label _label_2)
      (`SceneComponent.SetVisibility` (`self.Grenade`) false false)
      (`SceneComponent.SetVisibility` (`self.Gun`) false false)
      (`PrimitiveComponent.SetCollisionEnabled` (`self.Melee`) "QueryAndPhysics")
      (`/Engine/EditorBlueprintResources/StandardMacros.FlipFlop` :!label _label_3
        (:`A`
          (`|PlayMontage` _mesh "/Game/Frameworks/Assets/Characters/Animations/Stable_Sword_Inward_Slash_Montage.Stable_Sword_Inward_Slash_Montage"
            (:`OnCompleted`
              _)))
        (:`B`
          (`|PlayMontage` _mesh "/Game/Frameworks/Assets/Characters/Animations/Stabbing_Montage.Stabbing_Montage"
            (:`OnCompleted`
              _))))
      (if (`self.HoldingDownFire`)
        (`self.MeleeHold`)
        (else
          (`SceneComponent.SetVisibility` (`self.Gun`) true false)
          (`SceneComponent.SetVisibility` (`self.Melee`) false false)
          (`SceneComponent.SetVisibility` (`self.Grenade`) false false)
          (`PrimitiveComponent.SetCollisionEnabled` (`self.Melee`) "NoCollision")
          (set `self.Isattacking` false)))
      (elif (> (`self.Ammo`) 0)
        (`SceneComponent.SetVisibility` (`self.Gun`) true false)
        (`SceneComponent.SetVisibility` (`self.Melee`) false false)
        (`SceneComponent.SetVisibility` (`self.Grenade`) false false)
        (`|PlayMontage` (`self.Mesh`) "/Game/Frameworks/Assets/Characters/Meshes/Pose_Fire_Montage1.Pose_Fire_Montage1" :!label _label_4
          (:`OnCompleted`
            (`KismetSystemLibrary.Delay` (select `int` (`self.index`) :`0` 0.0 :`1` 0.0 :`2` 5.0 :!type "Float (single-precision)"))
            (if (`self.HoldingDownFire`)
              (`self.Refire`)
              (else
                (set `self.Isattacking` false)))))
        (else
          (goto _label_2))))))

(event `MeleeHold`
  (goto _label_3))

(event `Refire`
  (goto _label_4))

(event `FireGun`
  (bind _ammo (`self.Ammo`))
  (bind _aim (`self.Aim`))
  (bind _returnvalue (`SceneComponent.K2_GetComponentRotation` _aim))
  (bind _returnvalue_2 (`KismetMathLibrary.MakeTransform` (+ (`SceneComponent.K2_GetComponentLocation` _aim) (`KismetMathLibrary.GreaterGreater_VectorRotator` (`self.ProjectileOffset`) _returnvalue)) _returnvalue))
  ;[1 1 1] Fire Bullets
  (if (> _ammo 0)
    (set `self.Ammo` (`KismetMathLibrary.Clamp` (- _ammo 1) 0 (`self.Ammo_Max`)))
    (switch `int` (`self.index`)
      (:`0`
        (`|SpawnActorFromClass` "/Game/Frameworks/Blueprints/SpawnAssets/BP_Bullet.BP_Bullet_C" _returnvalue_2 "AlwaysSpawn" "MultiplyWithRoot" null self (`self.Bullet Damage`) null :!label _label_5))
      (:`1`
        (goto _label_5))
      (:`2`
        (`|SpawnActorFromClass` "/Game/Frameworks/Blueprints/SpawnAssets/BP_Granade.BP_Granade_C" _returnvalue_2 "Undefined" "MultiplyWithRoot" null self (`self.Explosion Damage`) 5 null)))
    (else
      (set `self.Isattacking` false))))

(fn `UserConstructionScript`
  (bind _index (`self.index`))
  (if (or (`self.IsPlayer`) (`self.IsTank`))
    (set `self.Tile` "Tank")
    (else
      (if (`self.IsRandom`)
        (set `self.index` (`KismetMathLibrary.RandomIntegerInRange` 0 2)))
      (`PrimitiveComponent.SetMaterial` (`self.Mesh`) 2 (select `int` (`self.index`) :`0` "/Game/Frameworks/Assets/Characters/Materials/Enemy_Red.Enemy_Red" :`1` "/Game/Frameworks/Assets/Characters/Materials/Black.Black" :`2` "/Game/Frameworks/Assets/Characters/Materials/Pants.Pants" :!type "MaterialInterface Object Reference"))
      (bind _output_get (set `self.HP` (select `int` _index :`0` 100.0 :`1` 150.0 :`2` 200.0)))
      (set `self.HP_Max` _output_get)
      (set `self.Tile` (select `int` _index :`0` "Private" :`1` "Corporal" :`2` "Sergeant" :!type "Text"))
      (`StaticMeshComponent.SetStaticMesh` (`self.Gun`) (select `int` (`self.index`) :`0` "/Game/Frameworks/Assets/Weapons/Meshes/AK.AK" :`1` "/Game/Frameworks/Assets/Weapons/Meshes/SMG.SMG" :`2` "/Game/Frameworks/Assets/Weapons/Meshes/GrenadeLauncher.GrenadeLauncher" :!type "StaticMesh Object Reference"))
      (`StaticMeshComponent.SetStaticMesh` (`self.Melee`) (select `int` (`self.index`) :`0` "/Game/Frameworks/Assets/Weapons/Meshes/Knife_1.Knife_1" :`1` "/Game/Frameworks/Assets/Weapons/Meshes/Knife_2.Knife_2" :`2` "/Game/Frameworks/Assets/Weapons/Meshes/Knife_2.Knife_2" :!type "StaticMesh Object Reference"))
      (bind _output_get_2 (set `self.Ammo` (select `int` (`self.index`) :`0` 300 :`1` 150 :`2` 5)))
      (set `self.Ammo_Max` _output_get_2))))