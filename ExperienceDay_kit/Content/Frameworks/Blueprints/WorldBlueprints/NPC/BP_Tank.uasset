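; Tank NPC character that fires a cannon, damages actors overlapping its box and explodes on death.
; FireCanno spawns a bullet at Arrow2 with smoke on a cooldown; its recoil launch has a zero vector and the aim-at-target node is unconnected.
; Damage lowers HP and plays a hit montage that blocks movement and further hits.
; Tick watches IsDead, set outside these graphs, then runs death montage, physics, explosion and removal.
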(event `self.Shoot`
  (`|PlayMontage` (`self.Mesh`) "/Game/Frameworks/Assets/Tank/Anim_Tank_Shoot_Montage1.Anim_Tank_Shoot_Montage1"))

(event `self.ReceiveTick`
  (params (DeltaSeconds :type "Float (single-precision)"))
  (`parent.ReceiveTick` DeltaSeconds)
  (if (`self.IsDead?`)
    (`/Engine/EditorBlueprintResources/StandardMacros.DoOnce` false
      (:`Completed`
        (`|PlayMontage` (`self.Mesh`) "/Game/Frameworks/Assets/Tank/Anim_Tank_Death_Montage.Anim_Tank_Death_Montage"
          (:`then`
            (`CharacterMovementComponent.SetMovementMode` (`self.CharacterMovement`) "MOVE_None" 0))
          (:`OnCompleted`
            (`self.Death` :!label _label))
          (:`OnInterrupted`
            (goto _label)))))))

(event `FireCanno`
  (bind _arrow2 (`self.Arrow2`))
  (bind (_returnvalue_location _returnvalue_rotation) (`KismetMathLibrary.BreakTransform` (`KismetMathLibrary.MakeTransform` (`SceneComponent.K2_GetComponentLocation` _arrow2) (`SceneComponent.K2_GetComponentRotation` _arrow2))))
  (if (not (`self.HasFired`))
    (`|SpawnActorFromClass` "/Game/Frameworks/Blueprints/SpawnAssets/BP_Bullet_Tank.BP_Bullet_Tank_C" (`KismetMathLibrary.MakeTransform` _returnvalue_location _returnvalue_rotation) "AlwaysSpawn" "MultiplyWithRoot" null self (`self.Bullet Damage`) null)
    (`ActorComponent.Activate` (`self.Land_Smoke`) true)
    (`self.LaunchCharacter` (* (0.0 0.0 0.0) -2000.0))
    (set `self.HasFired` true)
    (`KismetSystemLibrary.Delay` 5.0)
    (set `self.HasFired` false)))

(event `Death`
  (`PrimitiveComponent.SetSimulatePhysics` (`self.Mesh`) true)
  (`KismetSystemLibrary.Delay` 3.0)
  (`|SpawnActorFromClass` "/Game/Frameworks/Blueprints/SpawnAssets/BP_Boom.BP_Boom_C" (`KismetMathLibrary.MakeTransform` (`self.K2_GetActorLocation`)) "AlwaysSpawn" "MultiplyWithRoot" null null 50.0 null)
  (`self.Remove_Character`))

(event `self.Box.OnComponentBeginOverlap`
  (params (OverlappedComponent :type "PrimitiveComponent Object Reference") (OtherActor :type "Actor Object Reference") (OtherComp :type "PrimitiveComponent Object Reference") (OtherBodyIndex :type Integer) (bFromSweep :type Boolean) (SweepResult :type "HitResult Structure (by ref)"))
  (if (not (== OtherActor self))
    (`GameplayStatics.ApplyDamage` OtherActor 300.0)))

(event `self.ReceiveAnyDamage`
  (params (Damage :type "Float (single-precision)") (DamageType :type "DamageType Object Reference") (InstigatedBy :type "Controller Object Reference") (DamageCauser :type "Actor Object Reference"))
  (bind _hp (`self.HP`))
  (bind _charactermovement (`self.CharacterMovement`))
  ;[1 1 1] DamageApply
  (set `self.Damage Causer` DamageCauser)
  (if (not (`self.GettingHit`))
    (set `self.Isattacking` false)
    (if (> _hp 0.0)
      (set `self.HP` (`KismetMathLibrary.FClamp` (- _hp Damage) 0.0 (`self.HP_Max`)))
      (`|PlayMontage` (`self.Mesh`) "/Game/Frameworks/Assets/Tank/Anim_Tank_Hit_Montage.Anim_Tank_Hit_Montage"
        (:`then`
          (set `self.GettingHit` true)
          (`CharacterMovementComponent.SetMovementMode` _charactermovement "MOVE_None" 0))
        (:`OnCompleted`
          (set `self.GettingHit` false :!label _label_2)
          (`CharacterMovementComponent.SetMovementMode` _charactermovement "MOVE_Walking" 0))
        (:`OnInterrupted`
          (goto _label_2))))))

(fn `UserConstructionScript`
  (`parent.UserConstructionScript`))