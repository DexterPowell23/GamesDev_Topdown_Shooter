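; BP_Door is a lockable metal fence door that opens when the player enters its trigger box.
; A locked door consumes the player's key to unlock, with success or failure sounds.
; A timeline slides the fence open after a short delay and reverses to close it after a longer delay on exit or re-entry while open.
; A billboard sprite shows lock state, set in the construction script and every Tick.
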(event `self.ReceiveTick`
  (params (DeltaSeconds :type "Float (single-precision)"))
  (bind _billboard (`self.Billboard`))
  (if (`self.IsLocked?`)
    (`BillboardComponent.SetSprite` _billboard "/Game/Frameworks/Assets/Textures/Asset_61_2x.Asset_61_2x")
    (else
      (`BillboardComponent.SetSprite` _billboard "/Game/Frameworks/Assets/Textures/Asset_60_2x.Asset_60_2x"))))

(event `Open`
  (set `self.IsOpen?` true)
  (bind (_direction _moveback _open) (`Timeline|Open&Close` :!label _label)
    (:`Update`
      (`SceneComponent.K2_SetRelativeLocation` (`self.MetalFence`) (`KismetMathLibrary.MakeVector` _open _moveback) false false))))

(event `Close`
  (set `self.IsOpen?` false)
  (goto _label :!via `Reverse`))

(event `self.Box.OnComponentBeginOverlap`
  (params (OverlappedComponent :type "PrimitiveComponent Object Reference") (OtherActor :type "Actor Object Reference") (OtherComp :type "PrimitiveComponent Object Reference") (OtherBodyIndex :type Integer) (bFromSweep :type Boolean) (SweepResult :type "HitResult Structure (by ref)"))
  (bind _asbp_player (cast `/Game/Frameworks/Blueprints/Data/BP_Player` OtherActor))
  (if (`self.IsLocked?`)
    (if (`/Game/Frameworks/Blueprints/Data/BP_Player.IsPlayer` _asbp_player)
      (if (`/Game/Frameworks/Blueprints/Data/BP_Player.HasKey?` _asbp_player)
        (set `/Game/Frameworks/Blueprints/Data/BP_Player.HasKey?` false _asbp_player)
        (set `self.IsLocked?` false)
        (`GameplayStatics.PlaySoundAtLocation` "/Game/Frameworks/Sounds/CompileSuccess_Cue.CompileSuccess_Cue" (`self.K2_GetActorLocation`) (struct) 1.0 1.0 0.0 null null null null)
        (if (`self.IsOpen?`) :!label _label_2
          (`KismetSystemLibrary.Delay` 5.0)
          (`self.Close`)
          (else
            (`KismetSystemLibrary.Delay` 0.5)
            (`self.Open`)))
        (else
          (`GameplayStatics.PlaySoundAtLocation` "/Game/Frameworks/Sounds/CompileFailed_Cue.CompileFailed_Cue" (`self.K2_GetActorLocation`) (struct) 1.0 1.0 0.0 null null null null))))
    (else
      (goto _label_2))))

(event `self.Box.OnComponentEndOverlap`
  (params (OverlappedComponent :type "PrimitiveComponent Object Reference") (OtherActor :type "Actor Object Reference") (OtherComp :type "PrimitiveComponent Object Reference") (OtherBodyIndex :type Integer))
  (cast `/Game/Frameworks/Blueprints/Data/BP_Player` OtherActor)
  (if (`self.IsOpen?`)
    (`KismetSystemLibrary.Delay` 5.0)
    (`self.Close`)))

(fn `UserConstructionScript`
  (bind _billboard (`self.Billboard`))
  (if (`self.IsLocked?`)
    (`BillboardComponent.SetSprite` _billboard "/Game/Frameworks/Assets/Textures/Asset_61_2x.Asset_61_2x")
    (else
      (`BillboardComponent.SetSprite` _billboard "/Game/Frameworks/Assets/Textures/Asset_60_2x.Asset_60_2x"))))