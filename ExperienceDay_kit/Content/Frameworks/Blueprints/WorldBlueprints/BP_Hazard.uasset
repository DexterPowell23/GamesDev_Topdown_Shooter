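; BP_Hazard is a destructible world hazard prop that explodes when it takes any damage.
; Its construction script sets the mesh to an oil tank, exploding barrel or gas tank from the Hazard value, optionally picked at random from a list.
; The first damage event, guarded by a DoOnce, spawns a slightly enlarged BP_Boom explosion with set damage at its location, then destroys the hazard.
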(event `self.ReceiveAnyDamage`
  (params (Damage :type "Float (single-precision)") (DamageType :type "DamageType Object Reference") (InstigatedBy :type "Controller Object Reference") (DamageCauser :type "Actor Object Reference"))
  (`/Engine/EditorBlueprintResources/StandardMacros.DoOnce` false
    (:`Completed`
      (`|SpawnActorFromClass` "/Game/Frameworks/Blueprints/SpawnAssets/BP_Boom.BP_Boom_C" (`KismetMathLibrary.MakeTransform` (`self.K2_GetActorLocation`) (struct) (1.2 1.2 1.2)) "AlwaysSpawn" "MultiplyWithRoot" null null 50.0 null)
      (`self.K2_DestroyActor`))))

(fn `UserConstructionScript`
  (bind _staticmesh (`self.StaticMesh`))
  (if (`self.IsRandom?`)
    (set `self.Hazard` (`KismetArrayLibrary.Array_Random` (`self.ListRandom`))))
  (switch `/Game/Frameworks/Blueprints/Data/HazardTypes` (`self.Hazard`)
    (:`NewEnumerator0`
      (`StaticMeshComponent.SetStaticMesh` _staticmesh "/Game/Frameworks/Assets/Environment/Meshes/GasCan.GasCan"))
    (:`NewEnumerator1`
      (`StaticMeshComponent.SetStaticMesh` _staticmesh "/Game/Frameworks/Assets/Environment/Meshes/ExplodingBarrel.ExplodingBarrel"))
    (:`NewEnumerator2`
      (`StaticMeshComponent.SetStaticMesh` _staticmesh "/Game/Frameworks/Assets/Environment/Meshes/GasTank.GasTank"))))