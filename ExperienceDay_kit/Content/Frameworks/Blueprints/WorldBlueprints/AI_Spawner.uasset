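; AI_Spawner is a world Blueprint that periodically spawns AI-controlled enemies at its Arrow component's transform.
; A looping timer started on BeginPlay fires the Spawn event every few seconds.
; Spawn counts all BP_Enemies in the level and, below a small cap, creates an enemy and a separate AI_NPC_CON controller, which then possesses the new pawn.
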(event `self.ReceiveBeginPlay`
  (`KismetSystemLibrary.K2_SetTimerDelegate` (delegate `Spawn`) 5.0 true))

(event `Spawn`
  (bind _returnvalue (`SceneComponent.K2_GetComponentToWorld` (`self.Arrow`)))
  (bind _outactors (`GameplayStatics.GetAllActorsOfClass` "/Game/Frameworks/Blueprints/WorldBlueprints/BP_Enemies.BP_Enemies_C"))
  (if (not (> (`KismetArrayLibrary.Array_Length` _outactors) 5))
    (bind _returnvalue_2 (`|SpawnActorFromClass` "/Game/Frameworks/Blueprints/AI/AI_NPC_CON.AI_NPC_CON_C" _returnvalue "AlwaysSpawn" "MultiplyWithRoot" null null))
    (bind _returnvalue_3 (`|SpawnActorFromClass` "/Game/Frameworks/Blueprints/WorldBlueprints/BP_Enemies.BP_Enemies_C" _returnvalue "AlwaysSpawn" "MultiplyWithRoot" null 0 null false 0 50.0 40.0 100.0 false true 0 false null))
    (`Controller.Possess` _returnvalue_2 _returnvalue_3)))

(fn `UserConstructionScript`)