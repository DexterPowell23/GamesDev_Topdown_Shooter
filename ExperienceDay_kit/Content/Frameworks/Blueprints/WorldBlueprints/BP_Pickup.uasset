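; Pickup actor that grants health, ammo, a grenade or a key to a living BP_Player, excluding BP_Tank, on sphere overlap.
; The construction script sets mesh and label from the drop type, optionally randomized.
; Overlap applies the reward (health can raise max HP; keys require IsPlayer), then plays a sound and destroys the pickup.
; An Idle timeline with randomized play rate carries bob-and-spin logic, though no graph node starts it.
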(event `self.ReceiveBeginPlay`
  (`TimelineComponent.SetPlayRate` (`self.Idle`) (`KismetMathLibrary.RandomFloatInRange` 0.5 3.0)))

(event `self.Sphere.OnComponentBeginOverlap`
  (params (OverlappedComponent :type "PrimitiveComponent Object Reference") (OtherActor :type "Actor Object Reference") (OtherComp :type "PrimitiveComponent Object Reference") (OtherBodyIndex :type Integer) (bFromSweep :type Boolean) (SweepResult :type "HitResult Structure (by ref)"))
  (bind _asbp_player (cast `/Game/Frameworks/Blueprints/Data/BP_Player` OtherActor))
  (cast `/Game/Frameworks/Blueprints/WorldBlueprints/NPC/BP_Tank` OtherActor
    (:`CastFailed`
      (if (not (`/Game/Frameworks/Blueprints/Data/BP_Player.IsDead?` _asbp_player))
        (switch `/Game/Frameworks/Blueprints/Data/Pickup` (`self.Drop`)
          (:`NewEnumerator0`
            (bind _hp (`/Game/Frameworks/Blueprints/Data/BP_Player.HP` _asbp_player))
            (if (>= _hp 100.0)
              (bind _returnvalue (+ _hp 100.0))
              (bind _output_get (set `/Game/Frameworks/Blueprints/Data/BP_Player.HP_Max` _returnvalue _asbp_player))
              (set `/Game/Frameworks/Blueprints/Data/BP_Player.HP` _output_get _asbp_player)
              (else
                (set `/Game/Frameworks/Blueprints/Data/BP_Player.HP` (`KismetMathLibrary.FClamp` _returnvalue 0.0 (`/Game/Frameworks/Blueprints/Data/BP_Player.HP_Max` _asbp_player)) _asbp_player)))
            (`GameplayStatics.PlaySoundAtLocation` null (`self.K2_GetActorLocation`) (struct) 1.0 1.0 0.0 null null null null :!label _label)
            (`self.K2_DestroyActor`))
          (:`NewEnumerator1`
            (set `/Game/Frameworks/Blueprints/Data/BP_Player.Ammo` (`KismetMathLibrary.Clamp` (+ (`/Game/Frameworks/Blueprints/Data/BP_Player.Ammo` _asbp_player) 300) 0 (`/Game/Frameworks/Blueprints/Data/BP_Player.Ammo_Max` _asbp_player)) _asbp_player)
            (goto _label))
          (:`NewEnumerator2`
            (set `/Game/Frameworks/Blueprints/Data/BP_Player.Grenade_Current` (`KismetMathLibrary.Clamp` (+ (`/Game/Frameworks/Blueprints/Data/BP_Player.Grenade_Current` _asbp_player) 1) 0 (`/Game/Frameworks/Blueprints/Data/BP_Player.Grenade_Max` _asbp_player)) _asbp_player)
            (goto _label))
          (:`NewEnumerator3`
            (if (`/Game/Frameworks/Blueprints/Data/BP_Player.IsPlayer` _asbp_player)
              (set `/Game/Frameworks/Blueprints/Data/BP_Player.HasKey?` true _asbp_player)
              (goto _label))))))))

(fn `UserConstructionScript`
  (bind _drop (`self.Drop`))
  (bind _staticmesh (`self.StaticMesh`))
  (if (`self.IsRandom?`)
    (set `self.Drop` (`KismetArrayLibrary.Array_Random` (`self.Drop_Random`))))
  (switch `/Game/Frameworks/Blueprints/Data/Pickup` _drop
    (:`NewEnumerator0`
      (`StaticMeshComponent.SetStaticMesh` _staticmesh "/Game/Frameworks/Assets/Environment/Meshes/Health.Health"))
    (:`NewEnumerator1`
      (`StaticMeshComponent.SetStaticMesh` _staticmesh "/Game/Frameworks/Assets/Weapons/Meshes/AK.AK"))
    (:`NewEnumerator2`
      (`StaticMeshComponent.SetStaticMesh` _staticmesh "/Game/Frameworks/Assets/Weapons/Meshes/Grenade.Grenade"))
    (:`NewEnumerator3`
      (`StaticMeshComponent.SetStaticMesh` _staticmesh "/Game/Frameworks/Assets/Environment/Meshes/Key.Key")))
  (`TextRenderComponent.K2_SetText` (`self.TextRender`) (`|FormatText` "{Item} Drop Spawner" (`|GetEnumeratorNameAsString` _drop)))
  (if (`self.IsRandom?`)
    (`TextRenderComponent.K2_SetText` (`self.TextRender`) (`|FormatText` "{Item} Drop Spawner" "Random Item"))))